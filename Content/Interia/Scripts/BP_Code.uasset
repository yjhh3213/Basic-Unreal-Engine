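; BP_Code is a scripting test Blueprint that prints results of basic arithmetic, branch and loop logic on BeginPlay.
; A Sequence node prints FNumber plus SNumber via the Plus function, runs a branch fixed to true, then prints each loop index and an end message.
; The FNumber > SNumber comparison is left unconnected, and the Subtract function, which prints and returns a difference, is never called here.
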(event EventBeginPlay
  (Utilities|FlowControl|Sequence
    (:then_0
      ;[0.15 0.15 0.15 0.5] 두 수를 더해서 출력하는 코드
      (bind _returnv (CallFunction|Plus (Variables|Default|GetFNumber) (Variables|Default|GetSNumber)))
      (Development|PrintString (Utilities|String|ToString(Integer) _returnv)))
    (:then_1
      ;[0.15 0.15 0.15 0.5] 조건
      (if true
        (Development|PrintString "Num01이 크다")
        (else
          (Development|PrintString "num01이 작다"))))
    (:then_2
      (for _index (range 0 10)
        (Development|PrintString (Utilities|String|ToString(Integer) _index)))
      (Development|PrintString "End loop"))))

(event Collision|EventActorBeginOverlap
  (params (OtherActor :type Actor%20Object%20Reference)))

(event EventTick
  (params (DeltaSeconds :type Float%20%28single-precision%29)))

(fn ConstructionScript)

(fn Plus
  (params (Num01 :type Integer) (Num02 :type Integer))
  (return (+ Num01 Num02)))

(fn Subtract
  (params (Num01 :type Integer) (Num02 :type Integer))
  (bind _returnvalue (- Num01 Num02))
  (Development|PrintString (Utilities|String|ToString(Integer) _returnvalue))
  (return _returnvalue))