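; BP_EnemyManager is a spawner actor that periodically creates BP_Enemy actors at its own transform in the shooting game.
; Tick accumulates delta time and spawns an enemy once the elapsed time exceeds CreateTime.
; After each spawn it resets the timer and picks a new random interval of up to a few seconds, so enemies arrive at irregular gaps.
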(event EventBeginPlay)

(event Collision|EventActorBeginOverlap
  (params (OtherActor :type Actor%20Object%20Reference)))

(event EventTick
  (params (DeltaSeconds :type Float%20%28single-precision%29))
  ;[0.15 0.15 0.15 0.5] 현재시간을 흐르게 하는 코드
  (bind _output_get (Variables|Default|SetCurrTime (+ DeltaSeconds (Variables|Default|GetCurrTime))))
  ;[0.15 0.15 0.15 0.5] 1초마다 Enemy생성
  (if (> _output_get (Variables|Default|GetCreateTime))
    (Game|SpawnActorfromClass "/Game/Shooting/BluePrints/BP_Enemy.BP_Enemy_C" (Transformation|GetActorTransform) "Undefined" "MultiplyWithRoot" 0 0)
    ;[0.15 0.15 0.15 0.5] 현재시간을 초기화
    (Variables|Default|SetCurrTime 0.0)
    ;[0.15 0.15 0.15 0.5] 소환 시간을 랜덤하게
    (Variables|Default|SetCreateTime (Math|Random|RandomFloatinRange 0.0 5.0))))

(fn ConstructionScript)