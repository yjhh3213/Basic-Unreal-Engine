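; BP_Player is the player actor of a shooting game, moving on the Y/Z plane and firing BP_Bullet actors.
; BeginPlay adds the Enhanced Input mapping, and Tick moves it by normalized axis input times Speed without sweeping.
; Bullets spawn at FirePos on a repeating Tick timer and whenever IA_Fire starts.
; Any actor overlap opens GameOverMap, while the WBP_Shooting widget creation is left unconnected.
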(event Input|EnhancedActionEvents|EnhancedInputActionIA_Fire
  (params (ActionValue :type Boolean) (ElapsedSeconds :type Float%20%28double-precision%29) (TriggeredSeconds :type Float%20%28double-precision%29) (InputAction :type Input%20Action%20Object%20Reference :default "/Game/Shooting/Input/IA_Fire.IA_Fire"))
  (:Started
    ;[0.15 0.15 0.15 0.5] 총알을 FIrePos에서 생성하기
    (Game|SpawnActorfromClass "/Game/Shooting/BluePrints/BP_Bullet.BP_Bullet_C" (Transformation|GetWorldTransform (Variables|Default|GetFirePos)) "Undefined" "MultiplyWithRoot" 0 0)))

(event EventBeginPlay
  ;[0.15 0.15 0.15 0.5] Enchanced Input 초기 설정
  (Input|AddMappingContext (PlayerController|LocalPlayerSubsystems|GetEnhancedInputLocalPlayerSubsystem (Game|GetPlayerController 0)) "/Game/Shooting/Input/IMC_Input.IMC_Input" 0 "(bIgnoreAllPressedKeysUntilRelease=True,bForceImmediately=False,bNotifyUserSettings=False)"))

(event Collision|EventActorBeginOverlap
  (params (OtherActor :type Actor%20Object%20Reference))
  (Game|OpenLevel(byName) "GameOverMap"))

(event EventTick
  (params (DeltaSeconds :type Float%20%28single-precision%29))
  ;[0.15 0.15 0.15 0.5] 이동공식(P = P0+ vt)
  (Transformation|SetActorLocation (+ (* DeltaSeconds (* (Math|Vector|Normalize (Math|Vector|MakeVector 0.0 (Input|EnhancedActionValues|GetIA_Horizontal) (Input|EnhancedActionValues|GetIA_Vertical))) (Variables|Default|Getspeed))) (Transformation|GetActorLocation)) false false)
  ;[0.15 0.15 0.15 0.5] 0.3초마다 자동발사
  (bind _output_get (Variables|Default|SetCurrTime (+ DeltaSeconds (Variables|Default|GetCurrTime))))
  (if (> _output_get (Variables|Default|GetCreatTime))
    (Game|SpawnActorfromClass "/Game/Shooting/BluePrints/BP_Bullet.BP_Bullet_C" (Transformation|GetWorldTransform (Variables|Default|GetFirePos)) "Undefined" "MultiplyWithRoot" 0 0)
    (Variables|Default|SetCurrTime 0.0)))

(fn ConstructionScript)