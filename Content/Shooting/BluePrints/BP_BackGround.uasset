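; BP_BackGround is a scrolling background actor for the shooting game.
; Each tick it moves along its negative up vector at Speed, scaled by delta time.
; When its Z drops below a fixed lower limit, it jumps up by a fixed offset, so it recycles for continuous scrolling.
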(event EventBeginPlay)

(event Collision|EventActorBeginOverlap
  (params (OtherActor :type Actor%20Object%20Reference)))

(event EventTick
  (params (DeltaSeconds :type Float%20%28single-precision%29))
  ;[0.15 0.15 0.15 0.5] 이동공식(P = P0+ vt)
  (Transformation|SetActorLocation (+ (* DeltaSeconds (* (* (Transformation|GetActorUpVector) (Math|Float|MakeLiteralFloat -1.0)) (Variables|Default|GetSpeed))) (Transformation|GetActorLocation)) false false)
  ;[0.15 0.15 0.15 0.5] 만약에 위치 Z 값이 -3000보다 작아지면 현재위치에서 위로 9000만큼 생성
  (if (< (.z (Transformation|GetActorLocation)) -3e+03)
    (Transformation|SetActorLocation (+ (Transformation|GetActorLocation) "0.000000,0.000000,9000.000000") false false)))

(fn ConstructionScript)