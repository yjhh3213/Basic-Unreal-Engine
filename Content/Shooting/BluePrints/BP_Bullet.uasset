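; BP_Bullet is the projectile of a shooting game that flies straight and scores points when it hits an enemy.
; Each Tick moves it along its up vector by Speed times delta time, setting the location without sweep.
; On overlap, it identifies enemies by an "Enemy" substring in the other actor's display name, adds score through BP_ShootingGameMode and destroys only itself.
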(event EventBeginPlay)

(event Collision|EventActorBeginOverlap
  (params (OtherActor :type Actor%20Object%20Reference))
  ;[0.15 0.15 0.15 0.5] 만약에 Enemy랑 부딪혔다면 점수를 올리자
  (if (Utilities|String|Contains (Utilities|GetDisplayName OtherActor) "Enemy")
    (bind _asbp_shooting_game_mode (Utilities|Casting|CastToBP_ShootingGameMode (Game|GetGameMode)))
    (Default|AddScore _asbp_shooting_game_mode 5)
    (Actor|DestroyActor)))

(event EventTick
  (params (DeltaSeconds :type Float%20%28single-precision%29))
  ;[0.15 0.15 0.15 0.5] 이동공식(P = P0+ vt)
  (Transformation|SetActorLocation (+ (* DeltaSeconds (* (Transformation|GetActorUpVector) (Variables|Default|GetSpeed))) (Transformation|GetActorLocation)) false false))

(fn ConstructionScript)