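; Game mode for the shooting game that tracks the current score and a persistent high score.
; On BeginPlay it creates the WBP_Shooting HUD widget and loads the saved best score into it.
; AddScore accumulates the current score and, when it beats the best, updates the high-score text and saves it.
; Persistence uses a BP_SaveTotalScore SaveGame object in a single named slot.
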(event EventBeginPlay
  ;[0.15 0.15 0.15 0.5] WIdget 생성 후 화면에 붙이기(Create a widget and paste it on  the screen)
  (bind _returnvalue (UserInterface|CreateWidget "/Game/Shooting/BluePrints/WBP_Shooting.WBP_Shooting_C"))
  (bind _output_get (Variables|Default|SetShooting _returnvalue))
  (UserInterface|Viewport|AddtoPlayerScreen _output_get)
  (CallFunction|LoadTotalScore))

(event EventTick
  (params (DeltaSeconds :type Float%20%28single-precision%29)))

(fn ConstructionScript)

(fn AddScore
  (params (ScoreValue :type Integer))
  ;[0.15 0.15 0.15 0.5] 현재 점수를 증가
  (bind _output_get (Variables|Default|SetCurrentScore (+ ScoreValue (Variables|Default|GetCurrentScore))))
  ;[0.15 0.15 0.15 0.5] 최고 점수 갱신
  (if (> _output_get (Variables|Default|GetTotalScore))
    (bind _output_get_2 (Variables|Default|SetTotalScore _output_get))
    (Rendering|Components|TextRender|SetText (Variables|/Game/Shooting/BluePrints/WBP_Shooting.WBP_Shooting_C|GetText_TotalScoreValue (Variables|Default|GetShooting)) (Utilities|Text|ToText(Integer) _output_get_2))
    (CallFunction|SaveTotalScore)))

(fn SaveTotalScore
  (bind _returnvalue (SaveGame|CreateSaveGameObject "/Game/Shooting/BluePrints/BP_SaveTotalScore.BP_SaveTotalScore_C"))
  (Variables|/Game/Shooting/BluePrints/BP_SaveTotalScore.BP_SaveTotalScore_C|SetTotalScoreData _returnvalue (Variables|Default|GetTotalScore))
  (SaveGame|SaveGametoSlot _returnvalue "TOTAL_SCORE"))

(fn LoadTotalScore
  (bind _returnvalue (SaveGame|LoadGamefromSlot "TOTAL_SCORE"))
  (bind _asbp_save_total_score (Utilities|Casting|CastToBP_SaveTotalScore _returnvalue))
  (Utilities|IsValid _asbp_save_total_score
    (:Is%20Valid
      (bind _output_get (Variables|Default|SetTotalScore (Variables|/Game/Shooting/BluePrints/BP_SaveTotalScore.BP_SaveTotalScore_C|GetTotalScoreData _asbp_save_total_score)))
      (Rendering|Components|TextRender|SetText (Variables|/Game/Shooting/BluePrints/WBP_Shooting.WBP_Shooting_C|GetText_TotalScoreValue (Variables|Default|GetShooting)) (Utilities|Text|ToText(Integer) _output_get)))))