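; BP_Enemy is a shooter enemy that flies in a straight line and explodes on contact.
; At BeginPlay a random roll against PerCent either aims and rotates it toward BP_Player or sends it along its downward axis, which is also the fallback without a player.
; Tick moves it by Direction and Speed.
; Overlapping any actor without "Destroy" in its name spawns an explosion, plays a sound and destroys only the enemy.
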(event OnComponentBeginOverlap(Box)
  (params (OverlappedComponent :type Primitive%20Component%20Object%20Reference) (OtherActor :type Actor%20Object%20Reference) (OtherComp :type Primitive%20Component%20Object%20Reference) (OtherBodyIndex :type Integer) (bFromSweep :type Boolean) (SweepResult :type Hit%20Result%20Structure%20%28by%20ref%29)))

(event OnComponentEndOverlap(Box)
  (params (OverlappedComponent :type Primitive%20Component%20Object%20Reference) (OtherActor :type Actor%20Object%20Reference) (OtherComp :type Primitive%20Component%20Object%20Reference) (OtherBodyIndex :type Integer)))

(event EventBeginPlay
  (if (> (Math|Random|RandomIntegerinRange 1 10) (Variables|Default|GetPerCent))
    ;[0.15 0.15 0.15 0.5] Find to Player and get Location
    (bind _returnvalue (Actor|GetActorOfClass "/Game/Shooting/BluePrints/BP_Player.BP_Player_C"))
    (Utilities|IsValid _returnvalue
      (:Is%20Valid
        ;[0.15 0.15 0.15 0.5] Enemy가 Player를 향하는 방향을 구해서 DIR에 설정
        (bind _output_get (Variables|Default|SetDirection (Math|Vector|Normalize (- (Transformation|GetActorLocation _returnvalue) (Transformation|GetActorLocation)))))
        ;[0.15 0.15 0.15 0.5] Actor의 방향을 플레이어의 방향으로 회전시키는 방법
        (Transformation|SetActorRotation (Math|Rotator|MakeRotfromZX (* _output_get (Math|Float|MakeLiteralFloat -1.0)) (Transformation|GetActorForwardVector))))
      (:Is%20Not%20Valid
        ;[0.15 0.15 0.15 0.5] 아래 방향으로 설정
        (Variables|Default|SetDirection (* (Transformation|GetActorUpVector) (Math|Float|MakeLiteralFloat -1.0)) :!label _label)))
    (else
      (goto _label))))

(event Collision|EventActorBeginOverlap
  (params (OtherActor :type Actor%20Object%20Reference))
  (if (not (Utilities|String|Contains (Utilities|GetDisplayName OtherActor) "Destroy"))
    (Utilities|FlowControl|Sequence
      (:then_0
        ;[0.15 0.15 0.15 0.5] Enemy가 Bullet, Player에 충돌시 파괴
        (Effects|SpawnEmitteratLocation "/Game/StarterContent/Particles/P_Explosion.P_Explosion" (Transformation|GetActorLocation)) ; particle System
      )
      (:then_1
        (Audio|PlaySound2D "/Game/StarterContent/Audio/Explosion01.Explosion01" 1.0 1.0 0.0 0 0) ; 사운드 재생
        (Actor|DestroyActor))
      (:then_3
        (Actor|DestroyActor)))))

(event EventTick
  (params (DeltaSeconds :type Float%20%28single-precision%29))
  ;[0.15 0.15 0.15 0.5] 이동공식(P = P0+ vt)
  (Transformation|SetActorLocation (+ (* DeltaSeconds (* (Variables|Default|GetDirection) (Variables|Default|GetSpeed))) (Transformation|GetActorLocation)) false false))

(fn ConstructionScript)